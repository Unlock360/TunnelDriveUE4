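; TunnelBP is an actor Blueprint that builds a tunnel mesh along its Spline component.
; The construction script calls トンネルのメッシュを生成する (generate tunnel mesh), which loops over spline segments to add Spline Mesh components.
; Each component takes its start and end from adjacent points' local-space locations and tangents, so it bends with the curve.
; The return sits inside the loop body, so only the first segment gets a mesh.
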(fn ConstructionScript
  (|トンネルのメッシュを生成する) ; Create Tunnel Mesh
)
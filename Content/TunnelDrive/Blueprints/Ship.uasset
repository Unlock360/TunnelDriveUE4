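; Player ship for the tunnel game, attached to a TunnelTracerBP parent actor that it caches on BeginPlay.
; Non-zero MoveRight input updates PlayerDegree through a math expression, which drives the ship's roll.
; The relative location is a fixed trace offset rotated by that same roll, so the ship circles the parent's X axis while banking to match.
; BeginPlay also applies the initial angle to place the ship.
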(event EventBeginPlay
  (|変数のキャッシュ) ; Cache Variables
  (|最初のShip位置を設定) ; Initialize Ship Location
)

(event Input|AxisEvents|InputAxisMoveRight
  (params (AxisValue :type Float%20%28single-precision%29))
  (|左右の入力 AxisValue) ; Input Left-Right Key
)

(fn ConstructionScript)

(fn UpdateLocationandRotation
  (params (Roll :type Float%20%28single-precision%29))
  (bind _returnvalue (Math|Rotator|MakeRotator Roll 0.0 0.0))
  (Transformation|SetActorRelativeRotation _returnvalue) ; Update Rotation
  (Transformation|SetActorRelativeLocation (Math|Vector|RotateVector (Variables|Const|GetTRACE_OFFSET) _returnvalue)) ; Update Lcation
)
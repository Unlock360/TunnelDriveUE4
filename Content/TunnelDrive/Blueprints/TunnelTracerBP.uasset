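; TunnelTracerBP is an actor that travels continuously along the spline of the level's TunnelBP, tracing the tunnel's path.
; On BeginPlay it finds that TunnelBP and caches its spline and length.
; Each tick it advances a distance by move speed, looping at the spline's end, and sets its location there.
; Its rotation eases toward the spline's direction through RInterpTo, so turns lag smoothly behind position.
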(event EventBeginPlay
  (|変数のキャッシュなど) ; Initialize(Cache Variables)
)

(event EventTick
  (params (DeltaSeconds :type Float%20%28single-precision%29))
  (|トンネルの移動と回転を更新 DeltaSeconds) ; Update Move and Rotation
)

(fn ConstructionScript)